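; Player-controlled hero pawn that handles walking, punching and mouse-click point placement.
; On BeginPlay it spawns a MousePointBP at its own location and shows the cursor; left clicks move that point to the Visibility trace hit under the cursor.
; Axis inputs move the hero relative to control yaw only, and the Punch input holds IsPunching true while pressed.
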(event `self.ReceiveBeginPlay`
  (bind _returnvalue (`|SpawnActorFromClass` "/Game/UI/MousePointBP.MousePointBP_C" (`KismetMathLibrary.Conv_VectorToTransform` (`self.K2_GetActorLocation`)) "Undefined" "OverrideRootScale"))
  (set `self.MouseClickPoint` _returnvalue)
  (set `PlayerController.bShowMouseCursor` true (`GameplayStatics.GetPlayerController` 0)))

(event `InputAction|LeftMouseClicked`
  (params (Key :type "Key Structure" :default "AnyKey"))
  (:`Pressed`
    (`self.K2_SetActorLocation` (`self.MouseClickPoint`) (`.Location` (`GameplayStatics.BreakHitResult` (`PlayerController.GetHitResultUnderCursorByChannel` (`GameplayStatics.GetPlayerController` 0) "TraceTypeQuery1" true))) false false)))

(event `InputAxis|MoveForward`
  (params (AxisValue :type "Float (single-precision)"))
  (`self.AddMovementInput` (`KismetMathLibrary.GetForwardVector` (`KismetMathLibrary.MakeRotator` 0.0 0.0 (.yaw (`self.GetControlRotation`)))) AxisValue))

(event `InputAxis|MoveRight`
  (params (AxisValue :type "Float (single-precision)"))
  (`self.AddMovementInput` (`KismetMathLibrary.GetRightVector` (`KismetMathLibrary.MakeRotator` 0.0 0.0 (.yaw (`self.GetControlRotation`)))) AxisValue))

(event `InputAction|Punch`
  (params (Key :type "Key Structure" :default "AnyKey"))
  (:`Pressed`
    (set `self.IsPunching` true))
  (:`Released`
    (set `self.IsPunching` false)))

(fn `UserConstructionScript`)